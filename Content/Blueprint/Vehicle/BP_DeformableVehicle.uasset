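; BP_DeformableVehicle is a physics-based vehicle Blueprint with rear wheel components, a Box component and a movement on/off flag.
; StartMovement and StopMovement only set IsMovementEnabled.
; Disconnected graph logic would apply acceleration torque to both rear wheels while enabled, or a delayed forward impulse to the Box.
; Tick is empty and neither drive path runs, so this graph applies no movement.
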(event `self.ReceiveTick`
  (params (DeltaSeconds :type "Float (single-precision)")))

(fn `StartMovement`
  (set `self.bIsMovementEnabled` true))

(fn `StopMovement`
  (set `self.bIsMovementEnabled` false))

(fn `UserConstructionScript`)