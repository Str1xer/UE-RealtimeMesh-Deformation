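; BP_Button is an interactable button that highlights on hover and notifies listeners when used.
; The construction script creates a dynamic instance of M_Button on its Sphere component.
; Hover events drive that instance's Color parameter, switching between orange when hovered and white when not.
; Interact calls the OnInteract dispatcher, leaving the button's effect to whatever binds to it.
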(event `OnHover`
  (`MaterialInstanceDynamic.SetVectorParameterValue` (`self.Material`) "Color" (struct :`R` 1.0 :`G` 0.621732 :`A` 1.0)))

(event `OnUnhover`
  (`MaterialInstanceDynamic.SetVectorParameterValue` (`self.Material`) "Color" (struct :`R` 1.0 :`G` 1.0 :`B` 1.0 :`A` 1.0)))

(event `Interact`
  (`self.OnInteract`))

(fn `UserConstructionScript`
  (bind _returnvalue (`PrimitiveComponent.CreateDynamicMaterialInstance` (`self.Sphere`) 0 "/Game/Material/M_Button.M_Button" "None"))
  (set `self.Material` _returnvalue))