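; BP_Stand is an interactive stand that spawns a DeformableActor at its root and offers Throw and Reset child-actor buttons.
; Throw adds a temporary static mesh at a random offset around the Scene component, blocking further throws until it is destroyed after a delay.
; Reset destroys CurrentActor and spawns a replacement, but does not store the new reference in CurrentActor.
; The construction script writes the Title into a text render.
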(event `OnReset`
  (`self.K2_DestroyActor` (`self.CurrentActor`))
  (`|SpawnActorFromClass` (`self.DeformableActor`) (`SceneComponent.K2_GetComponentToWorld` (`self.DefaultSceneRoot`)) "Undefined" "MultiplyWithRoot" null null))

(event `self.ReceiveBeginPlay`
  (bind _returnvalue (`|SpawnActorFromClass` (`self.DeformableActor`) (`SceneComponent.K2_GetComponentToWorld` (`self.DefaultSceneRoot`)) "Undefined" "MultiplyWithRoot" null null))
  (set `self.CurrentActor` _returnvalue)
  (bind _asbp_button (cast `/Game/Blueprint/Interaction/BP_Button` (`ChildActorComponent.ChildActor` (`self.ThrowButton`))))
  (add `/Game/Blueprint/Interaction/BP_Button.OnInteract` _asbp_button (delegate `OnThrow`))
  (bind _asbp_button_2 (cast `/Game/Blueprint/Interaction/BP_Button` (`ChildActorComponent.ChildActor` (`self.ResetButton`))))
  (add `/Game/Blueprint/Interaction/BP_Button.OnInteract` _asbp_button_2 (delegate `OnReset`)))

(event `OnThrow`
  (bind _returnvalue_location (`KismetMathLibrary.BreakTransform` (`SceneComponent.GetRelativeTransform` (`self.Scene`))))
  (if (`self.bCanSpawn`)
    (bind _returnvalue (`AddComponent|NODE_AddStaticMeshComponent-0` :`RelativeTransform` (`KismetMathLibrary.MakeTransform` (+ _returnvalue_location (* (`KismetMathLibrary.RandomUnitVector`) 50.0)))))
    (set `self.bCanSpawn` false)
    (`KismetSystemLibrary.Delay` 5.0)
    (`ActorComponent.K2_DestroyComponent` _returnvalue)
    (set `self.bCanSpawn` true)))

(fn `UserConstructionScript`
  (`TextRenderComponent.K2_SetText` (`self.TextRender2`) (`self.Title`)))