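; Prototype of cage-based mesh deformation that shows a static mesh's vertices as a point cloud of instanced meshes.
; On BeginPlay it reads both meshes, spawns a node component at each unique scaled cage vertex, and precomputes per-vertex weights against the cage.
; UpdateMesh rebuilds each point as the weighted sum of current node locations and batch-updates the HISM instances.
; Show and Hide toggle node visibility.
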(event `self.ReceiveBeginPlay`
  (`self.Init`)
  (for (_array_element _array_index) (`self.Vertices`)
    (bind _returnvalue (`CageDev.ComputeWeights` _array_element (`self.CageVertices`) (`self.CageFaces`)))
    (`KismetArrayLibrary.Array_Set` (`self.Weights`) _array_index (make `/Game/Blueprint/CageProto/FWeights` _returnvalue) true)))

(fn `ArrayToString`
  (params (Array :type "Array of Float (double-precision)"))
  (returns (string :type String))
  (locals (stringArray :type "Array of String"))
  (for _array_element Array
    (`KismetArrayLibrary.Array_Add` (`local.stringArray`) (`KismetStringLibrary.Conv_DoubleToString` _array_element)))
  (return (`KismetStringLibrary.JoinStringArray` (`local.stringArray`) ",  ")))

(fn `Hide`
  (for _array_element (`self.NodeComponents`)
    (`SceneComponent.SetVisibility` _array_element false false)))

(fn `Init`
  (locals (Triangles :type "Array of Integer") (NodesLocation :type "Array of Vector Structure"))
  (bind _cagesize (`self.CageSize`))
  (`KismetArrayLibrary.Array_Clear` (`self.CageFaces`))
  (bind (_vertices _triangles) (`KismetProceduralMeshLibrary.GetSectionFromStaticMesh` (`self.MainMesh`)))
  (set `self.Vertices` _vertices)
  (set `local.Triangles` _triangles)
  (for _array_element (`self.Vertices`)
    (`InstancedStaticMeshComponent.AddInstance` (`self.HierarchicalInstancedStaticMesh`) (`KismetMathLibrary.MakeTransform` _array_element (struct) (0.01 0.01 0.01)) false))
  (bind (_vertices_2 _triangles_2) (`KismetProceduralMeshLibrary.GetSectionFromStaticMesh` (`self.CageMesh`)))
  (for _array_element_2 _vertices_2
    (`KismetArrayLibrary.Array_AddUnique` (`local.NodesLocation`) (* _array_element_2 _cagesize)))
  (for _array_element_3 _triangles_2
    (`KismetArrayLibrary.Array_Add` (`self.CageFaces`) (`KismetArrayLibrary.Array_Find` (`local.NodesLocation`) (* (`|GetArrayItem` _vertices_2 _array_element_3) _cagesize))))
  (for _array_element_4 (`local.NodesLocation`)
    (bind _returnvalue (`AddComponent|NODE_AddStaticMeshComponent-6` :`RelativeTransform` (`KismetMathLibrary.MakeTransform` _array_element_4 (struct) (0.1 0.1 0.1))))
    (`KismetArrayLibrary.Array_Add` (`self.NodeComponents`) _returnvalue)
    (`KismetArrayLibrary.Array_Add` (`self.CageVertices`) _array_element_4)))

(fn `Show`
  (for _array_element (`self.NodeComponents`)
    (`SceneComponent.SetVisibility` _array_element true false)))

(fn `UpdateMesh`
  (locals (LocalVert :type "Array of Vector Structure") (NewPos :type "Vector Structure") (NewTransform :type "Array of Transform Structure"))
  (set `local.LocalVert` (`self.Vertices`))
  (for (_ _array_index) (`local.LocalVert`)
    (set `local.NewPos` (0.0 0.0 0.0))
    (for (_array_element _array_index_2) (`.Weights_3_1C7DCAB343BDF19EF68858898646B32C` (break `/Game/Blueprint/CageProto/FWeights` (`|GetArrayItem` (`self.Weights`) _array_index)))
      (set `local.NewPos` (+ (* _array_element (`SceneComponent.RelativeLocation` (`|GetArrayItem` (`self.NodeComponents`) _array_index_2))) (`local.NewPos`))))
    (`KismetArrayLibrary.Array_Add` (`local.NewTransform`) (`KismetMathLibrary.MakeTransform` (`local.NewPos`) (struct) (0.01 0.01 0.01))))
  (`InstancedStaticMeshComponent.BatchUpdateInstancesTransforms` (`self.HierarchicalInstancedStaticMesh`) 0 (`local.NewTransform`) false true false))

(fn `UserConstructionScript`
  (locals (NewLocalVar :type "LinearColor Structure" :default (struct :`R` 1.0 :`A` 1.0)) (NodesLocation :type "Array of Vector Structure") (Triangles :type "Array of Integer")))