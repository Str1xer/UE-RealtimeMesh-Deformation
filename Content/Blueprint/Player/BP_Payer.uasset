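; Player pawn with camera-relative floating movement that fires projectiles on left mouse click.
; Turn and look axes feed controller yaw and pitch, while move axes push FloatingPawnMovement along the camera's forward and right vectors.
; Each click spawns a scaled-down BP_Projectile at the pawn's transform and launches it by setting its Sphere's physics velocity along the camera's forward vector.
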(event `InputAxis|TurnRate`
  (params (AxisValue :type "Float (single-precision)"))
  (`self.AddControllerYawInput` AxisValue))

(event `InputAxis|LookUpRate`
  (params (AxisValue :type "Float (single-precision)"))
  (`self.AddControllerPitchInput` AxisValue))

(event `Key|LeftMouseButton`
  (params (Key :type "Key Structure"))
  (:`Pressed`
    (bind _returnvalue (`|SpawnActorFromClass` "/Game/Blueprint/Projectile/BP_Projectile.BP_Projectile_C" (`KismetMathLibrary.MakeTransform` (`self.K2_GetActorLocation`) (`self.K2_GetActorRotation`) (0.75 0.75 0.75)) "Undefined" "MultiplyWithRoot" null null))
    (`PrimitiveComponent.SetPhysicsLinearVelocity` (`/Game/Blueprint/Projectile/BP_Projectile.Sphere` _returnvalue) (* (`SceneComponent.GetForwardVector` (`self.Camera`)) 750.0) false "None")))

(event `InputAxis|MoveForward`
  (params (AxisValue :type "Float (single-precision)"))
  (`PawnMovementComponent.AddInputVector` (`self.FloatingPawnMovement`) (* AxisValue (`SceneComponent.GetForwardVector` (`self.Camera`))) false))

(event `InputAxis|MoveRight`
  (params (AxisValue :type "Float (single-precision)"))
  (`PawnMovementComponent.AddInputVector` (`self.FloatingPawnMovement`) (* AxisValue (`SceneComponent.GetRightVector` (`self.Camera`))) false))

(fn `UserConstructionScript`)